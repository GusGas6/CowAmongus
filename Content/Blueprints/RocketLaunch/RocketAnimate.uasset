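; Rocket actor that plays a launch sequence when RocketTakeOffEvent is called.
; The event plays a takeoff sound and world camera shake, then activates two Niagara components and a smoke particle.
; The RocketGoUp timeline raises the static mesh by lerping from its current relative location toward a point above it, so movement accumulates each update and depends on frame rate.
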(event Custom|RocketTakeOffEvent
  (bind _staticmesh (Variables|Default|GetStaticMesh))
  (bind _relativelocation (Variables|/Script/Engine.SceneComponent|GetRelativeLocation _staticmesh))
  (Audio|PlaySound2D "/Game/Sounds/TakeoffSound.TakeoffSound" 1.0 1.0 0.0 0 0)
  (Camera|PlayWorldCameraShake "/Game/Blueprints/RocketLaunch/RocketCameraShake.RocketCameraShake_C" (Transformation|GetActorLocation) 5e+03 5e+03)
  (Components|Activation|Activate (Variables|Default|GetNiagara) false)
  (bind _rockettrack (Timeline|RocketGoUp PlayFromStart)
    (:Update
      (Transformation|SetRelativeLocation (Variables|Default|GetStaticMesh) (Math|Vector|Lerp(Vector) _relativelocation (+ _relativelocation "0.000000,0.000000,150.000000") _rockettrack) false false))))

(event EventBeginPlay)

(event Collision|EventActorBeginOverlap
  (params (OtherActor :type Actor%20Object%20Reference)))

(event EventTick
  (params (DeltaSeconds :type Float%20%28single-precision%29)))

(fn ConstructionScript)