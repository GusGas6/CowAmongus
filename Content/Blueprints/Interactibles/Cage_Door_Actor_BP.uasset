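; Cage door actor that slides open the first time the third-person player character overlaps it.
; On BeginPlay the door component snaps to its closed position.
; A DoOnce gate on the overlap triggers an eased MoveComponentTo to the open position, with GateClose_Cue played at the actor's location.
; Nothing closes the door again after it opens.
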(event Custom|DoorOpen
  (bind _door (Variables|Default|GetDoor))
  (Audio|PlaySoundatLocation "/Game/SFX/MetalDoor/GateClose_Cue.GateClose_Cue" (Transformation|GetActorLocation) "0, 0, 0" 1.0 1.0 0.0 0 0 0 0)
  (Components|MoveComponentTo _door (Variables|Default|GetOpenPosition) (Variables|/Script/Engine.SceneComponent|GetRelativeRotation _door) true true 1.4 false))

(event Custom|DoorClose
  (bind _door (Variables|Default|GetDoor))
  (Components|MoveComponentTo _door (Variables|Default|GetClosedPosition) (Variables|/Script/Engine.SceneComponent|GetRelativeRotation _door) false false 0.0 false))

(event EventBeginPlay
  (CallFunction|DoorClose))

(event Collision|EventActorBeginOverlap
  (params (OtherActor :type Actor%20Object%20Reference))
  (Utilities|Casting|CastToBP_ThirdPersonCharacter OtherActor)
  (Utilities|FlowControl|DoOnce false
    (:Completed
      (CallFunction|DoorOpen))))

(fn ConstructionScript)