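; An exit door actor that swings open the first time the third-person player character overlaps it.
; BeginPlay instantly snaps both door components to the closed rotation, and a DoOnce on the overlap triggers the eased one-second opening.
; MoveComponentTo drives both parts, with only Door targeting OpenRotation while Door1 has no explicit target rotation.
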(event Custom|DoorOpen
  (bind _door (Variables|Default|GetDoor))
  (bind _door1 (Variables|Default|GetDoor1))
  (Utilities|FlowControl|Sequence
    (:then_0
      (Components|MoveComponentTo _door1 (Variables|/Script/Engine.SceneComponent|GetRelativeLocation _door1) "0, 0, 0" true true 1.0 false))
    (:then_1
      (Components|MoveComponentTo _door (Variables|/Script/Engine.SceneComponent|GetRelativeLocation _door) (Variables|Default|GetOpenRotation) true true 1.0 false))))

(event Custom|DoorClose
  (bind _door1 (Variables|Default|GetDoor1))
  (bind _door (Variables|Default|GetDoor))
  (bind _closedrotation (Variables|Default|GetClosedRotation))
  (Utilities|FlowControl|Sequence
    (:then_0
      (Components|MoveComponentTo _door (Variables|/Script/Engine.SceneComponent|GetRelativeLocation _door) _closedrotation false false 0.0 false))
    (:then_1
      (Components|MoveComponentTo _door1 (Variables|/Script/Engine.SceneComponent|GetRelativeLocation _door1) _closedrotation false false 0.0 false))))

(event EventBeginPlay
  (CallFunction|DoorClose))

(event Collision|EventActorBeginOverlap
  (params (OtherActor :type Actor%20Object%20Reference))
  (Utilities|Casting|CastToBP_ThirdPersonCharacter OtherActor)
  (Utilities|FlowControl|DoOnce false
    (:Completed
      (CallFunction|DoorOpen))))

(fn ConstructionScript)