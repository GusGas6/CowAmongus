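; In-world TV that plays a one-time commander transmission cutscene when the player character first leaves its overlap area.
; The camera blends to the TV, then a delay-timed sequence swaps screen materials and plays the incoming alert, commander voiceline, static and turn-off sound before blending back to the player.
; While the commander talks, a self-restarting timeline pulses the TV mesh's scale to fake speech.
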(event Custom|TVTalking
  (Variables|Default|SetTVActive true)
  (if (Variables|Default|GetTVActive) :!label _label
    (bind _newtrack_0 (Timeline|Timeline PlayFromStart)
      (:Update
        (Transformation|SetRelativeScale3D (Variables|Default|GetTV) (Math|Vector|Lerp(Vector) "1.000000,1.000000,1.000000" "1.100000,1.050000,1.200000" _newtrack_0)))
      (:Finished
        (Utilities|FlowControl|DelayUntilNextTick)
        (goto _label)))))

(event Custom|BeginTV
  (bind _static (Variables|Default|GetStatic))
  (bind _tv (Variables|Default|GetTV))
  (Audio|Components|Audio|Stop _static)
  (Rendering|Material|SetMaterial _tv 0 "/Game/Materials/TV/TransmissionScreen_Mat.TransmissionScreen_Mat")
  (Audio|PlaySound2D "/Game/SFX/Commander/IncomingTransmission.IncomingTransmission" 1.0 1.0 0.0 0 0)
  (Utilities|FlowControl|Delay 2.8)
  (Audio|PlaySound2D "/Game/SFX/Commander/CommanderIntroVoiceline.CommanderIntroVoiceline" 1.0 1.0 0.0 0 0)
  (Rendering|Material|SetMaterial _tv 0 "/Game/Materials/TV/CommanderScreen_Mat.CommanderScreen_Mat")
  (CallFunction|TVTalking)
  (Utilities|FlowControl|Delay 6.0)
  (Rendering|Material|SetMaterial _tv 0 "/Game/Materials/TV/402107790_STATIC_NOISE_Mat.402107790_STATIC_NOISE_Mat")
  (Audio|Components|Audio|Play _static 0.0)
  (CallFunction|StopTalking)
  (Utilities|FlowControl|Sequence
    (:then_0
      (Utilities|FlowControl|Delay 0.5)
      (Audio|Components|Audio|Stop _static)
      (Rendering|Material|SetMaterial _tv 0 "/Engine/EngineDebugMaterials/BlackUnlitMaterial.BlackUnlitMaterial")
      (bind _asbp_third_person_character (Utilities|Casting|CastToBP_ThirdPersonCharacter (Game|GetPlayerCharacter 0)))
      (Game|Player|SetViewTargetwithBlend (Game|GetPlayerController 0) _asbp_third_person_character 1.5 "VTBlend_Linear" 0.0 false))
    (:then_1
      (Audio|PlaySound2D "/Game/SFX/Commander/TVTurnOff.TVTurnOff" 1.0 1.0 0.0 0 0))))

(event Custom|StopTalking
  (Variables|Default|SetTVActive false)
  (bind _newtrack_0 (Timeline|Timeline Stop)
    (:Update
      (Transformation|SetRelativeScale3D (Variables|Default|GetTV) (Math|Vector|Lerp(Vector) "1.000000,1.000000,1.000000" "1.100000,1.050000,1.200000" _newtrack_0)))
    (:Finished
      (Utilities|FlowControl|DelayUntilNextTick)
      (if (Variables|Default|GetTVActive)
        (Timeline|Timeline PlayFromStart)))))

(event Collision|EventActorEndOverlap
  (params (OtherActor :type Actor%20Object%20Reference))
  (Utilities|Casting|CastToBP_ThirdPersonCharacter OtherActor)
  (Utilities|FlowControl|DoOnce false
    (:Completed
      (Variables|Default|SetTVActive true)
      (Game|Player|SetViewTargetwithBlend (Game|GetPlayerController 0) self 1.5 "VTBlend_Linear" 0.0 false)
      (Utilities|FlowControl|Delay 2.3)
      (CallFunction|BeginTV))))

(fn ConstructionScript)