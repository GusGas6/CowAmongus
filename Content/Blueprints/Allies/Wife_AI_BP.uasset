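; Captive wife ally who is freed when the player overlaps her, then follows them by repeatedly moving to the ground traced beneath the player.
; Any damage ragdolls her with an impulse away from the causer, while her capsule tracks the spine bone; the first death flags the player and triggers brief slow motion.
; HideWife toggles an animated cardboard box once freed.
; RespawnWife restores her mesh and returns her to her captured start point.
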(event Custom|Death
  (params (Damage :type Float%20%28double-precision%29) (DamageCauser :type Actor%20Object%20Reference))
  (bind _mesh (Variables|Character|GetMesh))
  (bind _mesh_2 (Variables|Character|GetMesh))
  ;[1 1 1] Wife Death
  (Physics|SetSimulatePhysics _mesh true)
  (Variables|/Script/Engine.SkeletalMeshComponent|SetbPauseAnims _mesh true)
  (Physics|AddImpulse _mesh_2 (* (Math|Vector|GetUnitDirection(Vector) (Transformation|GetActorLocation DamageCauser) (Transformation|GetActorLocation)) Damage 1e+03) "None" false)
  (Transformation|DetachFromComponent _mesh_2 "KeepRelative" "KeepRelative" "KeepRelative" true)
  (Physics|SetEnableGravity (Variables|Collision|GetCapsuleComponent) false)
  (Variables|Default|SetDEAD true)
  (Utilities|FlowControl|Sequence
    (:then_0
      (Utilities|FlowControl|DoOnce false
        (:Completed
          (bind _asbp_third_person_character (Utilities|Casting|CastToBP_ThirdPersonCharacter (Game|GetPlayerCharacter 0)))
          (Variables|/Game/Blueprints/BP_ThirdPersonCharacter.BP_ThirdPersonCharacter_C|SetWifeDead _asbp_third_person_character true)
          (Utilities|Time|SetGlobalTimeDilation 0.1)
          (Class|GameplayStatics|SetGlobalPitchModulation 0.1 0.0)
          (Utilities|FlowControl|Delay 0.2)
          (Utilities|Time|SetGlobalTimeDilation 1.0)
          (Class|GameplayStatics|SetGlobalPitchModulation 1.0 0.0))))
    (:then_1
      (Transformation|SetWorldLocationAndRotation (Variables|Collision|GetCapsuleComponent) (.location (Transformation|GetBoneTransform (Variables|Character|GetMesh) "spine_05" "RTS_World")) "0, 0, 0" false true :!label _label)
      (if (Variables|Default|GetDEAD)
        (Utilities|FlowControl|DelayUntilNextTick)
        (goto _label)))))

(event Custom|FollowPlayer
  ;[1 1 1] FollowPlayer
  (if (Variables|Default|GetFollowingPlayer)
    (bind _asbp_third_person_character (Utilities|Casting|CastToBP_ThirdPersonCharacter (Game|GetPlayerCharacter 0)))
    (bind _outhit (Collision|LineTraceByChannel (Transformation|GetActorLocation _asbp_third_person_character) (- (Transformation|GetActorLocation _asbp_third_person_character) "0.000000,0.000000,10000.000000") "TraceTypeQuery1" false 0 "None"))
    (AI|AIMoveTo self (.Location (Collision|BreakHitResult _outhit)) 0 3e+02 false
      (:OnSuccess
        _)
      (:OnFail
        (Utilities|FlowControl|DelayUntilNextTick)))
    (CallFunction|FollowPlayer)))

(event Custom|RespawnWife
  (bind _mesh (Variables|Character|GetMesh))
  (bind _mesh_2 (Variables|Character|GetMesh))
  (Variables|Default|SetFollowingPlayer false)
  (Variables|Default|SetCaptured true)
  (Physics|SetSimulatePhysics _mesh_2 false)
  (Variables|Default|SetDEAD false)
  (Variables|/Script/Engine.SkeletalMeshComponent|SetbPauseAnims _mesh_2 false)
  (Transformation|Teleport (Variables|Default|GetRespawnLocation) (Variables|Default|GetRespawnRotation))
  (Transformation|AttachComponentToComponent _mesh (Variables|Collision|GetCapsuleComponent) "None" "SnapToTarget" "SnapToTarget" "SnapToTarget" true)
  (Components|MoveComponentTo _mesh "0.000000,0.000000,-92.632159" "0.000000,270.000000,0.000000" false false 0.0 false))

(event Custom|Freed
  ;[1 1 1] Whenplayer near, be free
  (Variables|Default|SetCaptured false)
  (Variables|Default|SetFollowingPlayer true)
  (CallFunction|FollowPlayer)
  (bind _asbp_third_person_character (Utilities|Casting|CastToBP_ThirdPersonCharacter (Game|GetPlayerCharacter 0)))
  (Variables|/Game/Blueprints/BP_ThirdPersonCharacter.BP_ThirdPersonCharacter_C|SetHasWife _asbp_third_person_character true))

(event Custom|HideWife
  ;[1 1 1] Hide Wife
  (if (not (Variables|Default|GetCaptured))
    (Utilities|FlowControl|FlipFlop
      (:A
        (Utilities|FlowControl|Sequence
          (:then_0
            (Development|SetHiddeninGame (Variables|Default|GetCardboard%20Box) false false)
            (Utilities|FlowControl|DoOnce false :!label _label
              (:Completed
                (bind _newtrack_0 (Timeline|Timeline PlayFromStart)
                  (:Update
                    (Transformation|SetRelativeScale3D (Variables|Default|GetCardboard%20Box) (Math|Vector|Lerp(Vector) "0, 0, 0" "1.192500,1.192500,1.192500" _newtrack_0))
                    (Transformation|SetRelativeLocation (Variables|Default|GetCardboard%20Box) (Math|Vector|Lerp(Vector) (Variables|Default|GetCardboxSpawnPosition) (Variables|Default|GetCardboxEquipPosition) _newtrack_0) false false))))))
          (:then_1
            (bind _newtrack_0_2 (Timeline|Timeline_0 Stop)
              (:Update
                (Transformation|SetRelativeScale3D (Variables|Default|GetCardboard%20Box) (Math|Vector|Lerp(Vector) "0, 0, 0" "1.192500,1.192500,1.192500" _newtrack_0_2))
                (Transformation|SetRelativeLocation (Variables|Default|GetCardboard%20Box) (Math|Vector|Lerp(Vector) (Variables|Default|GetCardboxEquipPosition) (Variables|Default|GetCardboxSpawnPosition) 0.0) false false))
              (:Finished
                (Development|SetHiddeninGame (Variables|Default|GetCardboard%20Box) true false))))))
      (:B
        (Utilities|FlowControl|Sequence
          (:then_0
            (Timeline|Timeline Stop))
          (:then_1
            (Timeline|Timeline_0 ReverseFromEnd))
          (:then_2
            (Utilities|FlowControl|Delay 0.3)
            (goto _label Reset)))))))

(event EventBeginPlay
  ;[1 1 1] Set respawn location
  (Variables|Default|SetRespawnRotation (Transformation|GetActorRotation))
  (Variables|Default|SetRespawnLocation (Transformation|GetActorLocation)))

(event Collision|EventActorBeginOverlap
  (params (OtherActor :type Actor%20Object%20Reference))
  ;[1 1 1] Whenplayer near, be free
  (Utilities|Casting|CastToBP_ThirdPersonCharacter OtherActor)
  (CallFunction|Freed))

(event Game|Damage|EventAnyDamage
  (params (Damage :type Float%20%28single-precision%29) (DamageType :type Damage%20Type%20Object%20Reference) (InstigatedBy :type Controller%20Object%20Reference) (DamageCauser :type Actor%20Object%20Reference))
  ;[1 1 1] IfHurt, die
  (CallFunction|Death Damage DamageCauser))

(fn ConstructionScript)