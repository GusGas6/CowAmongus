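; Floating UFO enemy that patrols and tractor-beams the player up to damage them.
; A timeline lerps it between four patrol points with randomized pauses, while a looping MoveComponentTo bobs the mesh.
; A downward trace each tick grounds the detection capsule; overlapping it halts patrol, reveals beam visuals and repeatedly launches the player toward the UFO.
; Sphere contact deals damage and ends the pull; ForgetPlayer, uncalled here, resumes patrol and resets visuals.
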(event OnComponentBeginOverlap(Capsule)
  (params (OverlappedComponent :type Primitive%20Component%20Object%20Reference) (OtherActor :type Actor%20Object%20Reference) (OtherComp :type Primitive%20Component%20Object%20Reference) (OtherBodyIndex :type Integer) (bFromSweep :type Boolean) (SweepResult :type Hit%20Result%20Structure%20%28by%20ref%29))
  ;[1 1 1] Collision
  (bind _asbp_third_person_character (Utilities|Casting|CastToBP_ThirdPersonCharacter OtherActor))
  (Variables|/Script/Engine.MovementComponent|SetVelocity (Variables|/Script/Engine.Character|GetCharacterMovement _asbp_third_person_character) "0, 0, 0")
  (Rendering|Components|Decal|SetDecalMaterial (Variables|Default|GetDecal) "/Game/Materials/LightCone/Circle_Light_Mat1.Circle_Light_Mat1")
  (Variables|Default|SetBeamingPlayer true)
  (CallFunction|StopPatrolling)
  (Development|SetHiddeninGame (Variables|Default|GetChildActor5) false false))

(event OnComponentBeginOverlap(Sphere)
  (params (OverlappedComponent :type Primitive%20Component%20Object%20Reference) (OtherActor :type Actor%20Object%20Reference) (OtherComp :type Primitive%20Component%20Object%20Reference) (OtherBodyIndex :type Integer) (bFromSweep :type Boolean) (SweepResult :type Hit%20Result%20Structure%20%28by%20ref%29))
  ;[1 1 1] Collision
  (bind _asbp_third_person_character (Utilities|Casting|CastToBP_ThirdPersonCharacter OtherActor))
  (Game|Damage|ApplyDamage _asbp_third_person_character 1.0 0 self)
  (Niagara|SpawnSystematLocation "/Game/Blueprints/DamageActors/BloodHit_P.BloodHit_P" (Transformation|GetActorLocation _asbp_third_person_character))
  (Variables|Default|SetBeamingPlayer false))

(event Custom|ForgetPlayer
  ;[1 1 1] Collision
  ;;[1 1 1] ForgetPlayer
  (Variables|Default|SetBeamingPlayer false)
  (CallFunction|Patrolling)
  (Rendering|Components|Decal|SetDecalMaterial (Variables|Default|GetDecal) "/Game/Materials/LightCone/Circle_Light_Mat.Circle_Light_Mat")
  (Development|SetHiddeninGame (Variables|Default|GetChildActor5) true false))

(event Custom|IdleBreathing
  (bind _returnvalue (Math|Random|RandomFloatinRange 0.8 1.4))
  (bind _staticmesh (Variables|Default|GetStaticMesh))
  (bind _relativelocation (Variables|/Script/Engine.SceneComponent|GetRelativeLocation _staticmesh))
  (bind _relativerotation (Variables|/Script/Engine.SceneComponent|GetRelativeRotation _staticmesh))
  ;[1 1 1] BreathingAnim
  (Components|MoveComponentTo _staticmesh (+ _relativelocation "0.000000,0.000000,25.000000") _relativerotation true true _returnvalue false :!label _label)
  (Components|MoveComponentTo _staticmesh (+ _relativelocation "0.000000,0.000000,-25.000000") _relativerotation true true _returnvalue false)
  (goto _label))

(event Custom|StopIdleBreathing
  (bind _returnvalue (Math|Random|RandomFloatinRange 0.8 1.4))
  (bind _staticmesh (Variables|Default|GetStaticMesh))
  (bind _relativelocation (Variables|/Script/Engine.SceneComponent|GetRelativeLocation _staticmesh))
  (bind _relativerotation (Variables|/Script/Engine.SceneComponent|GetRelativeRotation _staticmesh))
  ;[1 1 1] BreathingAnim
  (Components|MoveComponentTo _staticmesh (+ _relativelocation "0.000000,0.000000,-25.000000") _relativerotation true true _returnvalue false) ; enters at Stop
)

(event Custom|Patrolling
  ;[1 1 1] Patrolling
  (Utilities|IsValid (Variables|Default|GetNextPatrolTarget)
    (:Is%20Valid
      (Variables|Default|SetOriginalLocation (Transformation|GetActorLocation))
      (Variables|Default|SetOriginalRotatar (Transformation|GetActorRotation))
      (if (not (Variables|Default|GetBeamingPlayer))
        (bind _newtrack_0 (Timeline|Timeline PlayFromStart)
          (:Update
            (Transformation|SetActorLocation (Math|Vector|Lerp(Vector) (Variables|Default|GetOriginalLocation) (Transformation|GetActorLocation (Variables|Default|GetNextPatrolTarget)) _newtrack_0) false false))
          (:Finished
            (Utilities|FlowControl|Delay (+ (Math|Random|RandomFloatinRange 0.0 2.0) (Variables|Default|GetLingerTimer)))
            (if (>= (Variables|Default|GetPatrolNumber) 3)
              (Variables|Default|SetPatrolNumber 0)
              (else
                (Variables|Default|SetPatrolNumber (+ (Variables|Default|GetPatrolNumber) 1))))
            (switch int (Variables|Default|GetPatrolNumber)
              (:0
                (Variables|Default|SetNextPatrolTarget (Variables|Default|GetPatrolPointA)))
              (:1
                (Variables|Default|SetNextPatrolTarget (Variables|Default|GetPatrolPointB)))
              (:2
                (Variables|Default|SetNextPatrolTarget (Variables|Default|GetPartolPointC)))
              (:3
                (Variables|Default|SetNextPatrolTarget (Variables|Default|GetPatrolPointD))))
            (CallFunction|Patrolling)))))))

(event Custom|StopPatrolling
  ;[1 1 1] Patrolling
  (bind _newtrack_0 (Timeline|Timeline Stop)
    (:Update
      (Transformation|SetActorLocation (Math|Vector|Lerp(Vector) (Variables|Default|GetOriginalLocation) (Transformation|GetActorLocation (Variables|Default|GetNextPatrolTarget)) _newtrack_0) false false))
    (:Finished
      (Utilities|FlowControl|Delay (+ (Math|Random|RandomFloatinRange 0.0 2.0) (Variables|Default|GetLingerTimer)))
      (if (>= (Variables|Default|GetPatrolNumber) 3)
        (Variables|Default|SetPatrolNumber 0)
        (else
          (Variables|Default|SetPatrolNumber (+ (Variables|Default|GetPatrolNumber) 1))))
      (switch int (Variables|Default|GetPatrolNumber)
        (:0
          (Variables|Default|SetNextPatrolTarget (Variables|Default|GetPatrolPointA)))
        (:1
          (Variables|Default|SetNextPatrolTarget (Variables|Default|GetPatrolPointB)))
        (:2
          (Variables|Default|SetNextPatrolTarget (Variables|Default|GetPartolPointC)))
        (:3
          (Variables|Default|SetNextPatrolTarget (Variables|Default|GetPatrolPointD))))
      (CallFunction|Patrolling))))

(event EventBeginPlay
  (CallFunction|IdleBreathing)
  (Variables|Default|SetNextPatrolTarget (Variables|Default|GetPatrolPointA))
  (Utilities|FlowControl|DelayUntilNextTick)
  (CallFunction|Patrolling))

(event EventTick
  (params (DeltaSeconds :type Float%20%28single-precision%29))
  (bind _returnvalue (Transformation|GetActorLocation))
  (bind _decal (Variables|Default|GetDecal))
  ;[1 1 1] CursedPlayerTrackingandDecal
  (Utilities|FlowControl|Sequence
    (:then_0
      (bind (_outhit _returnvalue_2) (Collision|LineTraceByChannel _returnvalue (- _returnvalue "0.000000,0.000000,10000.000000") "TraceTypeQuery1" false 0 "None"))
      (if _returnvalue_2
        (Development|SetHiddeninGame _decal false false)
        (Transformation|SetWorldLocation (Variables|Default|GetCapsule) (.Location (Collision|BreakHitResult _outhit)) false false)
        (else
          (Development|SetHiddeninGame _decal true false))))
    (:then_1
      (if (Variables|Default|GetBeamingPlayer)
        (bind _asbp_third_person_character (Utilities|Casting|CastToBP_ThirdPersonCharacter (Game|GetPlayerCharacter 0)))
        (Character|LaunchCharacter _asbp_third_person_character (* (Math|Vector|GetUnitDirection(Vector) (Transformation|GetActorLocation) (Transformation|GetActorLocation _asbp_third_person_character)) -2e+02) true true)
        (Utilities|FlowControl|DoOnce false :!label _label
          (:Completed
            (Audio|PlaySoundatLocation "/Game/SFX/UFO/UFO_Beam_Cue.UFO_Beam_Cue" (Transformation|GetActorLocation) "0, 0, 0" 1.0 1.0 0.0 0 0 0 0)))
        (else
          (goto _label Reset))))))

(fn ConstructionScript)

(fn BeginningtoForgetPlayer)