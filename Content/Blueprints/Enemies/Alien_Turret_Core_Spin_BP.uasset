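; Alien turret core Blueprint that spins up and back down using a RotatingMovement component.
; On BeginPlay it starts spinning, then calls StopSpinning after a fixed delay.
; A single timeline drives the rotation rate on one axis, playing forward to ramp up and in reverse to ease back down.
; The Spin and StopSpinning events also set a Spinning flag.
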(event Custom|Spin
  (Variables|Default|SetSpinning true)
  (bind _newtrack_0 (Timeline|Timeline PlayFromStart)
    (:Update
      (Variables|/Script/Engine.RotatingMovementComponent|SetRotationRate (Variables|Default|GetRotatingMovement) (Math|Rotator|MakeRotator (Math|Float|Lerp 0.0 2e+03 _newtrack_0) 0.0 0.0)))))

(event Custom|StopSpinning
  (Variables|Default|SetSpinning false)
  (bind _newtrack_0 (Timeline|Timeline ReverseFromEnd)
    (:Update
      (Variables|/Script/Engine.RotatingMovementComponent|SetRotationRate (Variables|Default|GetRotatingMovement) (Math|Rotator|MakeRotator (Math|Float|Lerp 0.0 2e+03 _newtrack_0) 0.0 0.0)))))

(event EventBeginPlay
  (CallFunction|Spin)
  (Utilities|FlowControl|Delay 6.0)
  (CallFunction|StopSpinning))

(fn ConstructionScript)