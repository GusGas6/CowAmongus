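; Alien turret enemy that sweeps its searchlight between four patrol points, or waits stationary, until it spots the player.
; Tick traces the beam to place a decal and capsule; beam hits or line-of-sight-checked overlaps trigger aggro unless the player can't be spotted.
; Aggro turns the eye red, tracks the player and repeatedly fires projectiles with cone spread.
; A retriggerable delay driven by sphere-trace sight checks returns it to yellow-eyed patrol and idle bobbing.
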(event Custom|Spin
  ;[1 1 1] spin
)

(event Custom|StopSpinning
  ;[1 1 1] spin
)

(event Custom|ForceSpotPlayer
  (bind _returnvalue (Game|GetPlayerCharacter 0))
  ;[1 1 1] CursedPlayerTrackingandDecal
  (bind _asbp_third_person_character (Utilities|Casting|CastToBP_ThirdPersonCharacter (Game|GetPlayerCharacter 0)))
  (if (not (Variables|/Game/Blueprints/BP_ThirdPersonCharacter.BP_ThirdPersonCharacter_C|GetCannotBeSpotted _asbp_third_person_character))
    ;[1 1 1] Spotplayer
    (Variables|Default|SetFollowingPlayer true)
    (bind _asbp_third_person_character_2 (Utilities|Casting|CastToBP_ThirdPersonCharacter (Game|GetPlayerCharacter 0)))
    (Development|SetHiddeninGame (Variables|/Game/Blueprints/BP_ThirdPersonCharacter.BP_ThirdPersonCharacter_C|GetDecal _asbp_third_person_character_2) false false)
    (Development|SetHiddeninGame (Variables|Default|GetDecal) true false)
    (CallFunction|Aggro)
    (Utilities|FlowControl|DoOnce false
      (:Completed
        (Utilities|Casting|CastToBP_ThirdPersonCharacter _returnvalue)
        (Game|SpawnActorfromClass "/Game/Blueprints/PlayerAbilities/EnemyGroupAggroBubble_BP.EnemyGroupAggroBubble_BP_C" (Math|Transform|MakeTransform (Transformation|GetActorLocation _returnvalue) "0, 0, 0" "1.000000,1.000000,1.000000") "Undefined" "MultiplyWithRoot" 0 0)))))

(event Custom|BeginningToForgetPlayer
  ;[1 1 1] ForgetPlayerAfterXSeconds
  (Utilities|FlowControl|DoOnce false
    (:Completed
      (Utilities|FlowControl|RetriggerableDelay (Variables|Default|GetForgetDuration))
      (CallFunction|Peace))))

(event Custom|FireEvilEyes
  (bind _followingplayer (Variables|Default|GetFollowingPlayer))
  ;[1 1 1] fire
  (CallFunction|Spin)
  (Utilities|FlowControl|Delay (Variables|Default|GetTimerUntilFireWhenAggro))
  (bind _asbp_third_person_character (Utilities|Casting|CastToBP_ThirdPersonCharacter (Game|GetPlayerCharacter 0)))
  (if _followingplayer
    (Game|SpawnActorfromClass "/Game/Blueprints/DamageActors/EnemyProjectile_BP.EnemyProjectile_BP_C" (Math|Transform|MakeTransform (Transformation|GetWorldLocation (Variables|Default|GetSpotLight)) (Math|Conversions|RotationFromXVector (Math|Random|RandomUnitVectorinConeinDegrees (Math|Vector|GetUnitDirection(Vector) (Transformation|GetWorldLocation (Variables|Default|GetSkeletalMesh)) (Transformation|GetActorLocation _asbp_third_person_character)) 5.0)) "1.000000,1.000000,1.000000") "Undefined" "MultiplyWithRoot" 0 true 0)
    (Utilities|FlowControl|Delay (Variables|Default|GetFireRate))
    (if _followingplayer
      (CallFunction|RepeatFire)
      (else
        (CallFunction|StopSpinning)))))

(event Custom|RepeatFire
  (bind _followingplayer (Variables|Default|GetFollowingPlayer))
  ;[1 1 1] fire
  (bind _asbp_third_person_character (Utilities|Casting|CastToBP_ThirdPersonCharacter (Game|GetPlayerCharacter 0)))
  (if _followingplayer
    (Game|SpawnActorfromClass "/Game/Blueprints/DamageActors/EnemyProjectile_BP.EnemyProjectile_BP_C" (Math|Transform|MakeTransform (Transformation|GetWorldLocation (Variables|Default|GetSpotLight)) (Math|Conversions|RotationFromXVector (Math|Random|RandomUnitVectorinConeinDegrees (Math|Vector|GetUnitDirection(Vector) (Transformation|GetWorldLocation (Variables|Default|GetSkeletalMesh)) (Transformation|GetActorLocation _asbp_third_person_character)) 5.0)) "1.000000,1.000000,1.000000") "Undefined" "MultiplyWithRoot" 0 true 0)
    (Utilities|FlowControl|Delay (Variables|Default|GetFireRate))
    (if _followingplayer
      (CallFunction|RepeatFire)
      (else
        (CallFunction|StopSpinning)))))

(event Custom|IdleBreathing
  (bind _returnvalue (Math|Random|RandomFloatinRange 0.8 1.4))
  (bind _fakemover (Variables|Default|GetFakeMover))
  (bind _relativelocation (Variables|/Script/Engine.SceneComponent|GetRelativeLocation _fakemover))
  (bind _relativerotation (Variables|/Script/Engine.SceneComponent|GetRelativeRotation _fakemover))
  ;[1 1 1] BreathingAnim
  (Components|MoveComponentTo _fakemover (+ _relativelocation "0.000000,0.000000,25.000000") _relativerotation true true _returnvalue false :!label _label)
  (Components|MoveComponentTo _fakemover (+ _relativelocation "0.000000,0.000000,-25.000000") _relativerotation true true _returnvalue false)
  (goto _label))

(event Custom|StopIdleBreathing
  (bind _returnvalue (Math|Random|RandomFloatinRange 0.8 1.4))
  (bind _fakemover (Variables|Default|GetFakeMover))
  (bind _relativelocation (Variables|/Script/Engine.SceneComponent|GetRelativeLocation _fakemover))
  (bind _relativerotation (Variables|/Script/Engine.SceneComponent|GetRelativeRotation _fakemover))
  ;[1 1 1] BreathingAnim
  (Components|MoveComponentTo _fakemover (+ _relativelocation "0.000000,0.000000,-25.000000") _relativerotation true true _returnvalue false) ; enters at Stop
)

(event Custom|Patrolling
  (bind _skeletalmesh (Variables|Default|GetSkeletalMesh))
  ;[1 1 1] Patrolling
  (if (not (Variables|Default|GetFollowingPlayer))
    (Utilities|IsValid (Variables|Default|GetNextPatrolTarget)
      (:Is%20Valid
        (bind _newtrack_0 (Timeline|PatrolLookAt PlayFromStart)
          (:Update
            (Utilities|IsValid _skeletalmesh
              (:Is%20Valid
                (Transformation|SetRelativeRotation _skeletalmesh (Math|Rotator|Lerp(Rotator) (Transformation|GetWorldRotation _skeletalmesh) (Math|Rotator|MakeRotfromX (Math|Vector|GetUnitDirection(Vector) (- (Transformation|GetActorLocation (Variables|Default|GetNextPatrolTarget)) "0.000000,0.000000,-50.000000") (Transformation|GetWorldLocation (Variables|Default|GetSkeletalMesh)))) _newtrack_0) false false))))
          (:Finished
            (Utilities|FlowControl|Delay (+ (Math|Random|RandomFloatinRange 0.0 2.0) (Variables|Default|GetLingerTimer)))
            (if (>= (Variables|Default|GetPatrolNumber) 3)
              (Variables|Default|SetPatrolNumber 0)
              (else
                (Variables|Default|SetPatrolNumber (+ (Variables|Default|GetPatrolNumber) 1))))
            (switch int (Variables|Default|GetPatrolNumber)
              (:0
                (Variables|Default|SetNextPatrolTarget (Variables|Default|GetPatrolPointA)))
              (:1
                (Variables|Default|SetNextPatrolTarget (Variables|Default|GetPatrolPointB)))
              (:2
                (Variables|Default|SetNextPatrolTarget (Variables|Default|GetPartolPointC)))
              (:3
                (Variables|Default|SetNextPatrolTarget (Variables|Default|GetPatrolPointD))))
            (CallFunction|Patrolling)))))))

(event Custom|StartEvent
  ;[1 1 1] BeginPlay
  (CallFunction|IdleBreathing)
  (if (not (Variables|Default|GetStationaryUntilPlayerSpotted))
    (Utilities|FlowControl|Delay (Variables|Default|GetLingerTimer))))

(event Custom|StopPatrolling
  (bind _skeletalmesh (Variables|Default|GetSkeletalMesh))
  ;[1 1 1] Patrolling
  (bind _newtrack_0 (Timeline|PatrolLookAt Stop)
    (:Update
      (Utilities|IsValid _skeletalmesh
        (:Is%20Valid
          (Transformation|SetRelativeRotation _skeletalmesh (Math|Rotator|Lerp(Rotator) (Transformation|GetWorldRotation _skeletalmesh) (Math|Rotator|MakeRotfromX (Math|Vector|GetUnitDirection(Vector) (- (Transformation|GetActorLocation (Variables|Default|GetNextPatrolTarget)) "0.000000,0.000000,-50.000000") (Transformation|GetWorldLocation (Variables|Default|GetSkeletalMesh)))) _newtrack_0) false false))))
    (:Finished
      (Utilities|FlowControl|Delay (+ (Math|Random|RandomFloatinRange 0.0 2.0) (Variables|Default|GetLingerTimer)))
      (if (>= (Variables|Default|GetPatrolNumber) 3)
        (Variables|Default|SetPatrolNumber 0)
        (else
          (Variables|Default|SetPatrolNumber (+ (Variables|Default|GetPatrolNumber) 1))))
      (switch int (Variables|Default|GetPatrolNumber)
        (:0
          (Variables|Default|SetNextPatrolTarget (Variables|Default|GetPatrolPointA)))
        (:1
          (Variables|Default|SetNextPatrolTarget (Variables|Default|GetPatrolPointB)))
        (:2
          (Variables|Default|SetNextPatrolTarget (Variables|Default|GetPartolPointC)))
        (:3
          (Variables|Default|SetNextPatrolTarget (Variables|Default|GetPatrolPointD))))
      (CallFunction|Patrolling))))

(event Custom|Peace
  (bind _returnvalue (Game|GetPlayerCharacter 0))
  ;[1 1 1] AggroOrPeace
  (Variables|Default|SetFollowingPlayer false)
  (Variables|Default|SetPlayerSpotted false)
  (Variables|Default|SetFIRE false)
  (CallFunction|YellowEyes)
  (CallFunction|IdleBreathing)
  (CallFunction|Patrolling)
  (CallFunction|StopSpinning)
  (Utilities|FlowControl|Sequence
    (:then_0
      ;[1 1 1] Spotplayer
      (Utilities|FlowControl|DoOnce false) ; enters at Reset
    )
    (:then_1
      (bind _asbp_third_person_character (Utilities|Casting|CastToBP_ThirdPersonCharacter (Game|GetPlayerCharacter 0)))
      (Development|SetHiddeninGame (Variables|/Game/Blueprints/BP_ThirdPersonCharacter.BP_ThirdPersonCharacter_C|GetDecal _asbp_third_person_character) true false))))

(event Custom|Aggro
  ;[1 1 1] AggroOrPeace
  (Variables|Default|SetPlayerSpotted true)
  (Variables|Default|SetFollowingPlayer true)
  (CallFunction|RedEyes)
  (CallFunction|StopPatrolling)
  (CallFunction|StopIdleBreathing)
  (CallFunction|FireEvilEyes))

(event Custom|ForceForgetPlayer
  ;[1 1 1] ForgetPlayerAfterXSeconds
  (CallFunction|Peace))

(event Custom|YellowEyes
  ;[1 1 1] ManageColor
  (Rendering|Components|Light|SetLightColor (Variables|Default|GetSpotLight) "(R=1.000000,G=0.878595,B=0.000000,A=1.000000)" true)
  (Rendering|Material|SetMaterial (Variables|Default|GetCore) 0 "/Game/Materials/Alien_Search_Eye_Mat.Alien_Search_Eye_Mat")
  (Variables|Default|SetDecal%20Material "/Game/Materials/LightCone/Circle_Light_Mat2.Circle_Light_Mat2"))

(event Custom|RedEyes
  ;[1 1 1] ManageColor
  (Rendering|Components|Light|SetLightColor (Variables|Default|GetSpotLight) "(R=1.000000,G=0.027019,B=0.000000,A=1.000000)" true)
  (Rendering|Material|SetMaterial (Variables|Default|GetCore) 0 "/Game/Materials/Alien_Caught_Eye_Mat.Alien_Caught_Eye_Mat")
  (Variables|Default|SetDecal%20Material "/Game/Materials/LightCone/Red_Circle_Light_Mat3.Red_Circle_Light_Mat3"))

(event EventBeginPlay
  ;[1 1 1] BeginPlay
  (CallFunction|StartEvent)
  (CallFunction|YellowEyes)
  (Variables|Default|SetDecal%20Material "/Game/Materials/LightCone/Circle_Light_Mat2.Circle_Light_Mat2")
  (if (not (Variables|Default|GetStationaryUntilPlayerSpotted))
    (Variables|Default|SetNextPatrolTarget (Variables|Default|GetPatrolPointA))
    (CallFunction|Patrolling)))

(event EventTick
  (params (DeltaSeconds :type Float%20%28single-precision%29))
  (bind _decal (Variables|Default|GetDecal))
  (bind _capsule (Variables|Default|GetCapsule))
  ;[1 1 1] CursedPlayerTrackingandDecal
  (Utilities|FlowControl|Sequence
    (:then_0
      (bind (_outhit _returnvalue) (Collision|LineTraceByChannel (Transformation|GetWorldLocation (Variables|Default|GetSkeletalMesh)) (+ (Transformation|GetWorldLocation (Variables|Default|GetCone)) "0.000000,0.000000,300.000000") "TraceTypeQuery1" false 0 "None"))
      (if _returnvalue
        (Utilities|IsValid _decal
          (:Is%20Valid
            (if (Variables|Default|GetFollowingPlayer)
              (Transformation|SetWorldLocation _capsule (.Location (Collision|BreakHitResult _outhit)) false false :!label _label)
              (bind _asbp_third_person_character (Utilities|Casting|CastToBP_ThirdPersonCharacter (Game|GetPlayerCharacter 0)))
              (bind _outhit_2 (Collision|SphereTraceByChannel (Transformation|GetActorLocation) (Transformation|GetActorLocation _asbp_third_person_character) 25.0 "TraceTypeQuery1" false 0 "None"))
              (Utilities|Casting|CastToBP_ThirdPersonCharacter (.HitActor (Collision|BreakHitResult _outhit_2))
                (:then
                  (Utilities|FlowControl|Sequence
                    (:then_0
                      (bind _outhit_3 (Collision|LineTraceByChannel (Transformation|GetActorLocation _asbp_third_person_character) (- (Transformation|GetActorLocation _asbp_third_person_character) "0.000000,0.000000,100000.000000") "TraceTypeQuery1" false 0 "None"))
                      (Transformation|SetWorldLocation (Variables|Default|GetCapsule) (.Location (Collision|BreakHitResult _outhit_3)) false false)
                      (Utilities|FlowControl|Sequence :!label _label_2
                        (:then_0
                          (if (Variables|Default|GetFollowingPlayer)
                            (Utilities|FlowControl|DelayUntilNextTick)
                            (goto _label)))))
                    (:then_1
                      ;[1 1 1] ForgetPlayerAfterXSeconds
                      (Utilities|FlowControl|DoOnce false) ; enters at Reset
                    )))
                (:CastFailed
                  (CallFunction|BeginningtoForgetPlayer)
                  (goto _label_2)))
              (else
                (Transformation|SetWorldLocation _capsule (.Location (Collision|BreakHitResult _outhit)) false false)
                (Development|SetHiddeninGame _decal false false)
                (Utilities|Casting|CastToBP_ThirdPersonCharacter (.HitActor (Collision|BreakHitResult _outhit)))
                (CallFunction|ForceSpotPlayer)))))
        (elif (not (Variables|Default|GetFollowingPlayer))
          (Utilities|IsValid _decal
            (:Is%20Valid
              (Development|SetHiddeninGame _decal false false))))))
    (:then_1
      (if (Variables|Default|GetFollowingPlayer)
        (bind _asbp_third_person_character_2 (Utilities|Casting|CastToBP_ThirdPersonCharacter (Game|GetPlayerCharacter 0)))
        (Transformation|SetRelativeRotation (Variables|Default|GetSkeletalMesh) (Math|Rotator|MakeRotfromX (* (Math|Vector|GetUnitDirection(Vector) (Transformation|GetWorldLocation (Variables|Default|GetSkeletalMesh)) (Transformation|GetActorLocation _asbp_third_person_character_2)) -1.0)) false false)))))

(event Collision|EventActorBeginOverlap
  (params (OtherActor :type Actor%20Object%20Reference))
  (bind _returnvalue (Game|GetPlayerCharacter 0))
  ;[1 1 1] Spotplayer
  (bind _asbp_third_person_character (Utilities|Casting|CastToBP_ThirdPersonCharacter OtherActor))
  (bind _outhit (Collision|LineTraceByChannel (Transformation|GetActorLocation) (Transformation|GetActorLocation _asbp_third_person_character) "TraceTypeQuery1" false 0 "None"))
  (bind _asbp_third_person_character_2 (Utilities|Casting|CastToBP_ThirdPersonCharacter (.HitActor (Collision|BreakHitResult _outhit))))
  (if (not (Variables|/Game/Blueprints/BP_ThirdPersonCharacter.BP_ThirdPersonCharacter_C|GetCannotBeSpotted _asbp_third_person_character_2))
    (Variables|Default|SetFollowingPlayer true)
    (bind _asbp_third_person_character_3 (Utilities|Casting|CastToBP_ThirdPersonCharacter (Game|GetPlayerCharacter 0)))
    (Development|SetHiddeninGame (Variables|/Game/Blueprints/BP_ThirdPersonCharacter.BP_ThirdPersonCharacter_C|GetDecal _asbp_third_person_character_3) false false)
    (Development|SetHiddeninGame (Variables|Default|GetDecal) true false)
    (CallFunction|Aggro)
    (Utilities|FlowControl|DoOnce false
      (:Completed
        (Utilities|Casting|CastToBP_ThirdPersonCharacter _returnvalue)
        (Game|SpawnActorfromClass "/Game/Blueprints/PlayerAbilities/EnemyGroupAggroBubble_BP.EnemyGroupAggroBubble_BP_C" (Math|Transform|MakeTransform (Transformation|GetActorLocation _returnvalue) "0, 0, 0" "1.000000,1.000000,1.000000") "Undefined" "MultiplyWithRoot" 0 0)))))

(fn ConstructionScript)