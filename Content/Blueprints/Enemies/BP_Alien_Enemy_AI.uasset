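; Alien enemy AI that patrols up to four points or roams, investigates noises, and hunts the player with a shotgun.
; A capsule overlap plus line trace spots the player and spawns a group aggro bubble.
; Chasing re-traces line of sight every tick, leading to aim-and-fire or a last-known-location search before resuming patrol.
; Behavior runs on recursive AIMoveTo events and state flags, with eye and vision-cone materials showing alertness.
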(event OnComponentBeginOverlap(Eyesight)
  (params (OverlappedComponent :type Primitive%20Component%20Object%20Reference) (OtherActor :type Actor%20Object%20Reference) (OtherComp :type Primitive%20Component%20Object%20Reference) (OtherBodyIndex :type Integer) (bFromSweep :type Boolean) (SweepResult :type Hit%20Result%20Structure%20%28by%20ref%29))
  ;[1 1 1] Sight
  (bind _asbp_third_person_character (Utilities|Casting|CastToBP_ThirdPersonCharacter OtherActor))
  (if (not (Variables|/Game/Blueprints/BP_ThirdPersonCharacter.BP_ThirdPersonCharacter_C|GetCannotBeSpotted _asbp_third_person_character))
    (Utilities|IsValid (Variables|/Game/Blueprints/BP_ThirdPersonCharacter.BP_ThirdPersonCharacter_C|GetHurtBox _asbp_third_person_character)
      (:Is%20Valid
        (bind (_outhit _returnvalue) (Collision|LineTraceByChannel (Transformation|GetActorLocation) (Transformation|GetWorldLocation (Variables|/Game/Blueprints/BP_ThirdPersonCharacter.BP_ThirdPersonCharacter_C|GetHurtBox _asbp_third_person_character)) "TraceTypeQuery1" false 0 "None"))
        (if _returnvalue
          (Utilities|IsValid (.HitActor (Collision|BreakHitResult _outhit))
            (:Is%20Valid
              (Utilities|Casting|CastToBP_ThirdPersonCharacter (.HitActor (Collision|BreakHitResult _outhit)))
              (if (not (Variables|Default|GetChasingPlayer))
                (Game|SpawnActorfromClass "/Game/Blueprints/PlayerAbilities/EnemyGroupAggroBubble_BP.EnemyGroupAggroBubble_BP_C" (Math|Transform|MakeTransform (Transformation|GetActorLocation) "0, 0, 0" "1.000000,1.000000,1.000000") "Undefined" "MultiplyWithRoot" 0 0)
                (Variables|Default|SetPlayerSpotted true)
                (Variables|Default|SetHoldingGun true)
                (Audio|SpawnSoundatLocation "/Game/SFX/AlienSounds/AlienSpotted_Cue.AlienSpotted_Cue" (Transformation|GetWorldLocation (Variables|Character|GetMesh)) "0, 0, 0" 1.0 1.0 0.0 0 0)
                (if (Math|Random|RandomBoolwithWeight 0.1)
                  (Variables|Default|SetRudeGestureOnSpotPlayer true))
                (CallFunction|AggroSpeed)
                (CallFunction|RedEyes)
                (bind _asbp_third_person_character_2 (Utilities|Casting|CastToBP_ThirdPersonCharacter (Game|GetPlayerCharacter 0)))
                (AI|AIMoveTo self (Transformation|GetActorLocation _asbp_third_person_character_2) 0 5.0 false
                  (:then
                    (Utilities|FlowControl|DelayUntilNextTick)
                    (Variables|Default|SetRudeGestureOnSpotPlayer false)
                    (CallFunction|StopMovement)
                    (CallFunction|ChasePlayer)))))))))))

(event Custom|RandomRoam
  ;[1 1 1] RandomRoam
  (AI|AIMoveTo self (.RandomLocation (AI|Navigation|GetRandomReachablePointinRadius (Transformation|GetActorLocation) 9e+03 0 0)) 0 5.0 false
    (:OnSuccess
      _)
    (:OnFail
      _))
  (CallFunction|RandomRoam))

(event Custom|Patrol
  ;[1 1 1] PatrolBetweenActors
  (Utilities|IsValid (Variables|Default|GetPatrolActorA)
    (:Is%20Valid
      (if (not (Variables|Default|GetChasingPlayer))
        (AI|AIMoveTo self (Transformation|GetActorLocation (Variables|Default|GetPatrolActorA)) 0 5.0 false
          (:OnSuccess
            _)
          (:OnFail
            _))
        (Utilities|IsValid (Variables|Default|GetPatrolActorB)
          (:Is%20Valid
            (if (not (Variables|Default|GetChasingPlayer))
              (CallFunction|LookAroundNervous)
              (AI|AIMoveTo self (Transformation|GetActorLocation (Variables|Default|GetPatrolActorB)) 0 5.0 false
                (:OnSuccess
                  _)
                (:OnFail
                  _))
              (Utilities|IsValid (Variables|Default|GetPatrolActorC)
                (:Is%20Valid
                  (if (not (Variables|Default|GetChasingPlayer))
                    (CallFunction|LookAroundNervous)
                    (AI|AIMoveTo self (Transformation|GetActorLocation (Variables|Default|GetPatrolActorC)) 0 5.0 false
                      (:OnSuccess
                        _)
                      (:OnFail
                        _))
                    (Utilities|IsValid (Variables|Default|GetPatrolActorD)
                      (:Is%20Valid
                        (if (not (Variables|Default|GetChasingPlayer))
                          (CallFunction|LookAroundNervous)
                          (AI|AIMoveTo self (Transformation|GetActorLocation (Variables|Default|GetPatrolActorD)) 0 5.0 false
                            (:OnSuccess
                              _)
                            (:OnFail
                              _))
                          (if (not (Variables|Default|GetChasingPlayer))
                            (CallFunction|LookAroundNervous)
                            (CallFunction|Patrol))))
                      (:Is%20Not%20Valid
                        (CallFunction|RandomRoam)))))
                (:Is%20Not%20Valid
                  (CallFunction|RandomRoam)))))
          (:Is%20Not%20Valid
            (CallFunction|RandomRoam)))))
    (:Is%20Not%20Valid
      (CallFunction|RandomRoam))))

(event Custom|StopMovement
  ;[1 1 1] HandleMovementStopsAndResumes
  (Components|Activation|SetActive (Variables|Character|GetCharacterMovement) false false))

(event Custom|ResumeMovement
  (params (ReadyToFire :type Boolean))
  ;[1 1 1] HandleMovementStopsAndResumes
  (Components|Activation|SetActive (Variables|Character|GetCharacterMovement) true true)
  (Variables|Default|SetReadyToFire ReadyToFire)
  (if ReadyToFire
    (CallFunction|AggroSpeed)
    (else
      (CallFunction|PeacefulWalk))))

(event Custom|ChasePlayer
  (bind _returnvalue (Transformation|GetActorLocation))
  ;[1 1 1] PlayerChase
  (Variables|Default|SetChasingPlayer true)
  (Utilities|FlowControl|Sequence
    (:then_0
      (bind _asbp_third_person_character (Utilities|Casting|CastToBP_ThirdPersonCharacter (Game|GetPlayerCharacter 0)))
      (bind _outhit (Collision|LineTraceByChannel (Transformation|GetActorLocation _asbp_third_person_character) (- (Transformation|GetActorLocation _asbp_third_person_character) "0.000000,0.000000,10000.000000") "TraceTypeQuery1" false 0 "None"))
      (AI|AIMoveTo self (.Location (Collision|BreakHitResult _outhit)) 0 (Variables|Default|GetRangeBeforeFire) false
        (:then
          (Utilities|FlowControl|Delay 0.2)
          (if (Variables|Default|GetChasingPlayer)
            (CallFunction|ChasePlayer)))
        (:OnSuccess
          (if (Variables|Default|GetReadyToFire)
            (if (Variables|Default|GetPlayerIsInLineOfSight)
              (Utilities|FlowControl|DoOnce false
                (:Completed
                  (CallFunction|AimandFire)
                  (CallFunction|StopMovement)))
              (else
                (CallFunction|ForgetPlayer)))))))
    (:then_1
      (bind _asbp_third_person_character_2 (Utilities|Casting|CastToBP_ThirdPersonCharacter (Game|GetPlayerCharacter 0) :!label _label))
      (bind (_outhit_2 _returnvalue_2) (Collision|LineTraceByChannel _returnvalue (+ (Transformation|GetWorldLocation (Variables|/Game/Blueprints/BP_ThirdPersonCharacter.BP_ThirdPersonCharacter_C|GetHurtBox _asbp_third_person_character_2)) (* (Math|Vector|GetUnitDirection(Vector) _returnvalue (Transformation|GetWorldLocation (Variables|/Game/Blueprints/BP_ThirdPersonCharacter.BP_ThirdPersonCharacter_C|GetHurtBox _asbp_third_person_character_2))) 5e+04)) "TraceTypeQuery1" false 0 "None"))
      (Utilities|FlowControl|Sequence
        (:then_0
          (if (Variables|Default|GetChasingPlayer)
            (Utilities|FlowControl|DelayUntilNextTick)
            (goto _label)))
        (:then_1
          (if _returnvalue_2
            (bind _asbp_third_person_character_3 (Utilities|Casting|CastToBP_ThirdPersonCharacter (.HitActor (Collision|BreakHitResult _outhit_2)))
              (:then
                (if (Variables|/Game/Blueprints/BP_ThirdPersonCharacter.BP_ThirdPersonCharacter_C|GetCannotBeSpotted _asbp_third_person_character_3)
                  _
                  (else
                    (Variables|Default|SetPlayerIsInLineOfSight true)
                    (Variables|/Game/Blueprints/BP_ThirdPersonCharacter.BP_ThirdPersonCharacter_C|SetCantHide _asbp_third_person_character_3 true)
                    (Variables|Default|SetRangeBeforeFire (Variables|Default|GetShootingDistance))
                    (Variables|Default|SetPlayerLastKnownLocation (.Location (Collision|BreakHitResult _outhit_2)))
                    (goto _label_2 Reset))))
              (:CastFailed
                _))
            (Variables|Default|SetPlayerIsInLineOfSight false)
            (Utilities|FlowControl|Sequence
              (:then_0
                (Variables|Default|SetRangeBeforeFire 5.0)
                (Utilities|FlowControl|DoOnce false :!label _label_2
                  (:Completed
                    (Utilities|FlowControl|DelayUntilNextTick)
                    (CallFunction|ForgetPlayer))))
              (:then_1
                (bind _asbp_third_person_character_4 (Utilities|Casting|CastToBP_ThirdPersonCharacter (Game|GetPlayerCharacter 0)))
                (Variables|/Game/Blueprints/BP_ThirdPersonCharacter.BP_ThirdPersonCharacter_C|SetCantHide _asbp_third_person_character_4 false)))))))))

(event Custom|ForgetPlayer
  (bind _self self)
  (bind _playerlastknownlocation (Variables|Default|GetPlayerLastKnownLocation))
  (bind _randomlocation (AI|Navigation|GetRandomReachablePointinRadius _playerlastknownlocation 7e+02 0 0))
  ;[1 1 1] PlayerChase
  (Utilities|FlowControl|RetriggerableDelay (Variables|Default|GetTimeToForgetPlayerAndResumePatrol) :!label _label)
  (if (Variables|Default|GetPlayerIsInLineOfSight)
    (goto _label)
    (else
      (Variables|Default|SetChasingPlayer false)
      (AI|AIMoveTo _self _randomlocation 0 25.0 false
        (:OnSuccess
          _)
        (:OnFail
          _))
      (Utilities|FlowControl|Delay 1.0)
      (if (not (Variables|Default|GetChasingPlayer))
        (AI|AIMoveTo _self _randomlocation 0 25.0 false
          (:OnSuccess
            _)
          (:OnFail
            _))
        (Utilities|FlowControl|Delay 2.0)
        (if (not (Variables|Default|GetChasingPlayer))
          (AI|AIMoveTo _self _randomlocation 0 25.0 false
            (:OnSuccess
              _)
            (:OnFail
              _))
          (Utilities|FlowControl|Delay 2.0)
          (if (not (Variables|Default|GetChasingPlayer))
            (AI|AIMoveTo self _randomlocation 0 5.0 false
              (:OnSuccess
                _)
              (:OnFail
                _))
            (if (not (Variables|Default|GetChasingPlayer))
              (CallFunction|Patrol)
              (CallFunction|YellowEyes)
              (CallFunction|PeacefulWalk)
              (Variables|Default|SetHoldingGun false))))))))

(event Custom|ResetFire
  ;[1 1 1] PlayerChase
  (Utilities|FlowControl|DoOnce false) ; enters at Reset
)

(event Custom|AimAndFire
  ;[1 1 1] AimAndFire
  (Utilities|FlowControl|DoOnce false :!label _label
    (:Completed
      (Variables|Default|SetFiring true)
      (Variables|Default|SetStopAiming false)
      (Utilities|FlowControl|Sequence
        (:then_0
          (Utilities|FlowControl|Delay (Math|Random|RandomFloatinRange 1.0 1.3))
          (Variables|Default|SetStopAiming true)
          (Variables|Default|SetFIRE true)
          (Physics|AddRadialForce (Variables|Default|GetEyesight) (Transformation|GetWorldLocation (Variables|Default|GetSelfKnockbackOrigin)) 6e+03 6e+03 "RIF_Constant" true)
          (Utilities|FlowControl|Sequence
            (:then_0
              (Utilities|FlowControl|Delay 6.0)
              (Variables|Default|SetFiring false)
              (CallFunction|ResetFire)
              (Utilities|FlowControl|Sequence
                (:then_0
                  (goto _label Reset))
                (:then_1
                  (Variables|Default|SetRecovering true)
                  (if (Variables|Default|GetChasingPlayer)
                    (CallFunction|ChasePlayer)))))
            (:then_1
              (Utilities|FlowControl|DelayUntilNextTick)
              (Variables|Default|SetFIRE false))))
        (:then_1
          (bind _asbp_third_person_character (Utilities|Casting|CastToBP_ThirdPersonCharacter (Game|GetPlayerCharacter 0) :!label _label_2))
          (AI|AIMoveTo self (Transformation|GetActorLocation _asbp_third_person_character) 0 5.0 false
            (:then
              (if (not (Variables|Default|GetStopAiming))
                (if (not (Variables|Default|GetFIRE))
                  (Utilities|FlowControl|DelayUntilNextTick)
                  (goto _label_2))))))
        (:then_2
          (Audio|SpawnSoundatLocation "/Game/SFX/PrototypeSFX/Shotgun/ShotgunCockIn_Cue.ShotgunCockIn_Cue" (Transformation|GetActorLocation) "0, 0, 0" 1.0 1.0 0.0 0 0))))))

(event Custom|RandomLookAroundNervous
  ;[1 1 1] Random Look ARound while patrolling
  (Utilities|FlowControl|Delay (+ (Variables|Default|GetTimerBetweenRandomPause) (Math|Random|RandomFloatinRange 1e+01 35.0)))
  (Utilities|FlowControl|Sequence
    (:then_0
      (if (Math|Random|RandomBoolwithWeight 0.5)
        (Variables|Default|SetNervousLookARound true)
        (else
          (Variables|Default|SetPanicLookAround true)))
      (CallFunction|StopMovement)
      (if (Math|Random|RandomBoolwithWeight 0.1)
        (Audio|SpawnSoundatLocation "/Game/SFX/AlienSounds/AlienIdle_Cue.AlienIdle_Cue" (Transformation|GetWorldLocation (Variables|Character|GetMesh)) "0, 0, 0" 1.0 1.0 0.0 0 0))
      (Utilities|FlowControl|DelayUntilNextTick)
      (Variables|Default|SetNervousLookARound false)
      (Variables|Default|SetPanicLookAround false))
    (:then_1
      (Utilities|FlowControl|Delay 6.0)
      (CallFunction|RandomLookAroundNervous))))

(event Custom|FireGun
  (bind _bulletspawnpoint (Variables|Default|GetBulletSpawnPoint))
  (bind _mesh (Variables|Character|GetMesh))
  (bind _returnvalue (Math|Vector|GetForwardVector _bulletspawnpoint))
  (bind _returnvalue_2 (Transformation|GetWorldLocation _mesh))
  (bind _returnvalue_3 (Transformation|GetWorldLocation _bulletspawnpoint))
  ;[1 1 1] AimAndFire
  (Game|SpawnActorfromClass "/Game/Blueprints/DamageActors/EnemyProjectile_BP.EnemyProjectile_BP_C" (Math|Transform|MakeTransform _returnvalue_3 (Math|Conversions|RotationFromXVector _returnvalue) "1.000000,1.000000,1.000000") "Undefined" "MultiplyWithRoot" 0 false 0)
  (Utilities|FlowControl|Sequence
    (:then_0
      (for _index (range 0 7)
        (Game|SpawnActorfromClass "/Game/Blueprints/DamageActors/EnemyProjectile_BP.EnemyProjectile_BP_C" (Math|Transform|MakeTransform _returnvalue_3 (Math|Conversions|RotationFromXVector (Math|Random|RandomUnitVectorinConeinDegrees _returnvalue 15.0)) "1.000000,1.000000,1.000000") "Undefined" "MultiplyWithRoot" 0 false 0)))
    (:then_1
      (Utilities|FlowControl|DelayUntilNextTick)
      (Audio|SpawnSoundatLocation "/Game/SFX/PrototypeSFX/Shotgun_Fire_Cue.Shotgun_Fire_Cue" _returnvalue_2 "0, 0, 0" 1.0 1.0 0.0 0 0)
      (if (Math|Random|RandomBoolwithWeight 0.3)
        (Audio|SpawnSoundatLocation "/Game/SFX/AlienSounds/AlienHurt_Cue.AlienHurt_Cue" _returnvalue_2 "0, 0, 0" 1.0 1.0 0.0 0 0)))))

(event Custom|LookAroundNervous
  ;[1 1 1] Random Look ARound while patrolling
  (if (Math|Random|RandomBoolwithWeight 0.5)
    (Variables|Default|SetNervousLookARound true)
    (else
      (Variables|Default|SetPanicLookAround true)))
  (CallFunction|StopMovement)
  (if (Math|Random|RandomBoolwithWeight 0.1)
    (Audio|SpawnSoundatLocation "/Game/SFX/AlienSounds/AlienIdle_Cue.AlienIdle_Cue" (Transformation|GetWorldLocation (Variables|Character|GetMesh)) "0, 0, 0" 1.0 1.0 0.0 0 0))
  (Utilities|FlowControl|DelayUntilNextTick)
  (Variables|Default|SetNervousLookARound false)
  (Variables|Default|SetPanicLookAround false))

(event Custom|GroupAggro
  ;[1 1 1] Allows Groups to attack together
  (Utilities|FlowControl|Delay (Math|Random|RandomFloatinRange 0.5 1.5))
  (bind _asbp_third_person_character (Utilities|Casting|CastToBP_ThirdPersonCharacter (Game|GetPlayerCharacter 0)))
  (if (not (Variables|/Game/Blueprints/BP_ThirdPersonCharacter.BP_ThirdPersonCharacter_C|GetCannotBeSpotted _asbp_third_person_character))
    ;[1 1 1] Sight
    (if (not (Variables|Default|GetChasingPlayer))
      (Game|SpawnActorfromClass "/Game/Blueprints/PlayerAbilities/EnemyGroupAggroBubble_BP.EnemyGroupAggroBubble_BP_C" (Math|Transform|MakeTransform (Transformation|GetActorLocation) "0, 0, 0" "1.000000,1.000000,1.000000") "Undefined" "MultiplyWithRoot" 0 0)
      (Variables|Default|SetPlayerSpotted true)
      (Variables|Default|SetHoldingGun true)
      (Audio|SpawnSoundatLocation "/Game/SFX/AlienSounds/AlienSpotted_Cue.AlienSpotted_Cue" (Transformation|GetWorldLocation (Variables|Character|GetMesh)) "0, 0, 0" 1.0 1.0 0.0 0 0)
      (if (Math|Random|RandomBoolwithWeight 0.1)
        (Variables|Default|SetRudeGestureOnSpotPlayer true))
      (CallFunction|AggroSpeed)
      (CallFunction|RedEyes)
      (bind _asbp_third_person_character_2 (Utilities|Casting|CastToBP_ThirdPersonCharacter (Game|GetPlayerCharacter 0)))
      (AI|AIMoveTo self (Transformation|GetActorLocation _asbp_third_person_character_2) 0 5.0 false
        (:then
          (Utilities|FlowControl|DelayUntilNextTick)
          (Variables|Default|SetRudeGestureOnSpotPlayer false)
          (CallFunction|StopMovement)
          (CallFunction|ChasePlayer))))))

(event Custom|InvestigateNoise
  (params (NoiseLocation :type Vector))
  ;[1 1 1] NoiseHeard
  (Variables|Default|SetNoise%20Location NoiseLocation)
  (if (not (Variables|Default|GetPlayerIsInLineOfSight))
    (if (Variables|Default|GetHoldingGun)
      _
      (else
        (Variables|Default|SetHoldingGun true)
        (CallFunction|AggroSpeed)
        (AI|AIMoveTo self NoiseLocation 0 5.0 false
          (:then
            (Utilities|FlowControl|DelayUntilNextTick)
            (Variables|Default|SetRudeGestureOnSpotPlayer false)
            (CallFunction|StopMovement)))))
    (AI|AIMoveTo self (Variables|Default|GetNoise%20Location) 0 5.0 false
      (:OnSuccess
        _)
      (:OnFail
        _))
    (Utilities|FlowControl|Delay 1.0)
    (AI|AIMoveTo self (.RandomLocation (AI|Navigation|GetRandomReachablePointinRadius (Variables|Default|GetNoise%20Location) 1e+02 0 0)) 0 5.0 false
      (:OnSuccess
        _)
      (:OnFail
        _))
    (Utilities|FlowControl|Delay 1.0)
    (AI|AIMoveTo self (.RandomLocation (AI|Navigation|GetRandomReachablePointinRadius (Variables|Default|GetNoise%20Location) 1e+02 0 0)) 0 5.0 false
      (:OnSuccess
        _)
      (:OnFail
        _))
    (Utilities|FlowControl|Delay 1.0)
    (CallFunction|Patrol)))

(event Custom|GunEquip
  ;[1 1 1] TogglesActiveGun
  (Development|SetHiddeninGame (Variables|Default|GetGunOnBack_Mesh) true true)
  (Development|SetHiddeninGame (Variables|Default|GetGunHeld_Mesh) false true))

(event Custom|GunHolster
  ;[1 1 1] TogglesActiveGun
  (Development|SetHiddeninGame (Variables|Default|GetGunOnBack_Mesh) false true)
  (Development|SetHiddeninGame (Variables|Default|GetGunHeld_Mesh) true true)
  (Variables|Default|SetHoldingGun false)
  (Variables|Default|SetReadyToFire false)
  (if (Math|Random|RandomBoolwithWeight 0.25)
    (Audio|SpawnSoundatLocation "/Game/SFX/AlienSounds/AlienGuessItWasTheWind_Cue.AlienGuessItWasTheWind_Cue" (Transformation|GetWorldLocation (Variables|Character|GetMesh)) "0, 0, 0" 1.0 1.0 0.0 0 0)))

(event Custom|PeacefulWalk
  ;[1 1 1] SetAggroMovespeedAndEyes
  (Variables|/Script/Engine.CharacterMovementComponent|SetMaxWalkSpeed (Variables|Character|GetCharacterMovement) 1.5e+02))

(event Custom|AggroSpeed
  ;[1 1 1] SetAggroMovespeedAndEyes
  (Variables|/Script/Engine.CharacterMovementComponent|SetMaxWalkSpeed (Variables|Character|GetCharacterMovement) 4.5e+02))

(event Custom|ForceForgetPlayer
  ;[1 1 1] PlayerChase
  (Transformation|Teleport (Variables|Default|GetRespawnLocation) "0, 0, 0")
  (Variables|Default|SetChasingPlayer false)
  (Variables|Default|SetPlayerSpotted false)
  (Variables|Default|SetRecovering true)
  (Variables|Default|SetReadyToFire false)
  (Variables|Default|SetEquipGun false)
  (CallFunction|Patrol)
  (CallFunction|YellowEyes)
  (CallFunction|PeacefulWalk)
  (Variables|Default|SetHoldingGun false))

(event Custom|RedEyes
  ;[1 1 1] SetAggroMovespeedAndEyes
  (Rendering|Material|SetMaterial (Variables|Character|GetMesh) 1 "/Game/Materials/Alien_Caught_Eye_Mat.Alien_Caught_Eye_Mat")
  (Rendering|Components|Decal|SetDecalMaterial (Variables|Default|GetDecal) "/Game/Materials/LightCone/Vision_Light_Cone_Mat1.Vision_Light_Cone_Mat1"))

(event Custom|YellowEyes
  ;[1 1 1] SetAggroMovespeedAndEyes
  (Rendering|Material|SetMaterial (Variables|Character|GetMesh) 1 "/Game/Materials/Alien_Search_Eye_Mat.Alien_Search_Eye_Mat")
  (Rendering|Components|Decal|SetDecalMaterial (Variables|Default|GetDecal) "/Game/Materials/LightCone/Vision_Light_Cone_Mat.Vision_Light_Cone_Mat"))

(event EventBeginPlay
  (bind _eyesightdistance (Variables|Default|GetEyesightDistance))
  ;[1 1 1] OnBeginPlay = Patrol
  (Variables|Default|SetRespawnLocation (Transformation|GetActorLocation))
  (Variables|Default|SetRespawn%20Rotation (Transformation|GetActorRotation))
  (Variables|Default|SetShootingDistance (* _eyesightdistance 5.0))
  (Components|Capsule|SetCapsuleSize (Variables|Default|GetEyesight) (Variables|Default|GetEyesightWidth) _eyesightdistance true)
  (Utilities|FlowControl|Delay 2.0)
  (CallFunction|Patrol)
  (CallFunction|RandomLookAroundNervous)
  (if (Variables|Default|GetStationaryUntilPlayerSpotted)
    (CallFunction|StopMovement)))

(fn ConstructionScript)