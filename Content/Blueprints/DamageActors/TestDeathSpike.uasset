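; Test spike hazard actor that jabs a cone up and down and heavily damages any actor overlapping it.
; From BeginPlay, two latent MoveComponentTo calls loop endlessly, raising and lowering the cone by a fixed offset over short random durations.
; Actor overlap applies flat damage with the spike as causer, with no filter on the other actor or check on the cone's motion phase.
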(event EventBeginPlay
  (bind _returnvalue (Math|Random|RandomFloatinRange 0.1 0.2))
  (bind _cone (Variables|Default|GetCone))
  (bind _relativelocation (Variables|/Script/Engine.SceneComponent|GetRelativeLocation _cone))
  (bind _relativerotation (Variables|/Script/Engine.SceneComponent|GetRelativeRotation _cone))
  (Components|MoveComponentTo _cone (+ _relativelocation "0.000000,0.000000,35.000000") _relativerotation false false _returnvalue false :!label _label)
  (Components|MoveComponentTo _cone (+ _relativelocation "0.000000,0.000000,-35.000000") _relativerotation false false _returnvalue false)
  (goto _label))

(event Collision|EventActorBeginOverlap
  (params (OtherActor :type Actor%20Object%20Reference))
  (Game|Damage|ApplyDamage OtherActor 1e+02 0 self))

(fn ConstructionScript)