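; Enemy projectile that damages the player character or the Wife AI on hit and destroys itself after three seconds otherwise.
; A TurretBullet flag switches its Niagara trail to a red variant at spawn.
; Character hits play an impact sound, apply fixed damage, spawn blood and destroy the bullet.
; Projectile movement bounces play a ricochet sound and attach a temporary impact decal aligned to the surface normal.
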(event OnProjectileBounce(ProjectileMovement)
  (params (ImpactResult :type Hit%20Result%20Structure%20%28by%20ref%29) (ImpactVelocity :type Vector%20%28by%20ref%29 :default "0, 0, 0"))
  (bind (_bblockinghit _binitialoverlap _time _distance _location _impactpoint _normal _impactnormal _physmat _hitactor _hitcomponent) (Collision|BreakHitResult ImpactResult))
  (Audio|PlaySoundatLocation "/Game/SFX/Bullet/Ricochet/Ricochet_Cue.Ricochet_Cue" (Transformation|GetActorLocation) "0, 0, 0" 1.0 1.0 0.0 0 0 0 0)
  (Class|GameplayStatics|SpawnDecalAttached "/Game/Blueprints/DamageActors/bulletimpactdecal_Mat.bulletimpactdecal_Mat" "35.000000,35.000000,35.000000" _hitcomponent "None" _location (Math|Conversions|RotationFromXVector _normal) "KeepWorldPosition" 3e+01))

(event EventBeginPlay
  (if (Variables|Default|GetTurretBullet)
    (Class|NiagaraComponent|SetAsset (Variables|Default|GetBulletTrail_P) "/Game/Blueprints/DamageActors/BulletTrail_P_Red.BulletTrail_P_Red" true))
  (Utilities|FlowControl|Delay 3.0)
  (Actor|DestroyActor))

(event Collision|EventHit
  (params (MyComp :type Primitive%20Component%20Object%20Reference) (Other :type Actor%20Object%20Reference) (OtherComp :type Primitive%20Component%20Object%20Reference) (bSelfMoved :type Boolean) (HitLocation :type Vector :default "0, 0, 0") (HitNormal :type Vector :default "0, 0, 0") (NormalImpulse :type Vector :default "0, 0, 0") (Hit :type Hit%20Result%20Structure%20%28by%20ref%29))
  (bind _asbp_third_person_character (Utilities|Casting|CastToBP_ThirdPersonCharacter Other)
    (:then
      (Audio|PlaySoundatLocation "/Game/SFX/Bullet/BulletImpact_Cue.BulletImpact_Cue" (Transformation|GetActorLocation _asbp_third_person_character) "0, 0, 0" 1.0 1.0 0.0 0 0 0 0)
      (Game|Damage|ApplyDamage Other 3e+02 0 self)
      (Niagara|SpawnSystematLocation "/Game/Blueprints/DamageActors/BloodHit_P.BloodHit_P" HitLocation)
      (Actor|DestroyActor))
    (:CastFailed
      (bind _aswife_ai_bp (Utilities|Casting|CastToWife_AI_BP Other))
      (Audio|PlaySoundatLocation "/Game/SFX/Bullet/BulletImpact_Cue.BulletImpact_Cue" (Transformation|GetActorLocation _aswife_ai_bp) "0, 0, 0" 1.0 1.0 0.0 0 0 0 0)
      (Game|Damage|ApplyDamage _aswife_ai_bp 3e+02 0 self)
      (Niagara|SpawnSystematLocation "/Game/Blueprints/DamageActors/BloodHit_P.BloodHit_P" HitLocation)
      (Actor|DestroyActor))))

(fn ConstructionScript)