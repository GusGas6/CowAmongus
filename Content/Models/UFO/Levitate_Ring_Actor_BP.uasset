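; Levitation ring actor for a UFO model that animates a single ring mesh as soon as play begins.
; On BeginPlay it slides the mesh 100 units down in relative space with MoveComponentTo while a timeline shrinks it toward zero scale.
; The scale lerp reads the current scale on every update, so the shrink compounds.
; The actor is not destroyed afterward.
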(event EventBeginPlay
  (bind _staticmesh (Variables|Default|GetStaticMesh))
  (bind _staticmesh_2 (Variables|Default|GetStaticMesh))
  (Utilities|FlowControl|Sequence
    (:then_0
      (Components|MoveComponentTo _staticmesh (+ (Variables|/Script/Engine.SceneComponent|GetRelativeLocation _staticmesh) "0.000000,0.000000,-100.000000") (Variables|/Script/Engine.SceneComponent|GetRelativeRotation _staticmesh) false false 3.0 false))
    (:then_1
      (bind _newtrack_0 (Timeline|d PlayFromStart)
        (:Update
          (Transformation|SetRelativeScale3D _staticmesh_2 (Math|Vector|Lerp(Vector) (Variables|/Script/Engine.SceneComponent|GetRelativeScale3D _staticmesh_2) "0, 0, 0" _newtrack_0)))))))

(fn ConstructionScript)