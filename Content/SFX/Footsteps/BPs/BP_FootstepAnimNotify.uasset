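; Anim notify that plays surface-dependent footstep sounds for BP_ThirdPersonCharacter, staying silent while crouched.
; It traces downward from the actor, prints the hit's physical surface, and switches on it to play a cue at the actor's location.
; Rock is the fallback.
; Tile, Water and Puddle play the Snow, Tile and Water cues respectively, apparently misaligned, and the Puddle cue is never reached.
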(fn ReceivedNotify
  (params (MeshComp :type Skeletal%20Mesh%20Component%20Object%20Reference) (Animation :type Anim%20Sequence%20Base%20Object%20Reference) (EventReference :type Anim%20Notify%20Event%20Reference%20Structure%20%28by%20ref%29))
  (bind _returnvalue (Components|GetOwner MeshComp))
  (bind _returnvalue_2 (Transformation|GetActorLocation _returnvalue))
  (bind _asbp_third_person_character (Utilities|Casting|CastToBP_ThirdPersonCharacter _returnvalue))
  (if (not (AI|Components|NavMovement|IsCrouching (Variables|/Script/Engine.Character|GetCharacterMovement _asbp_third_person_character)))
    (bind (_outhit _returnvalue_3) (Collision|LineTraceByChannel _returnvalue_2 (+ _returnvalue_2 (* (Transformation|GetActorUpVector _returnvalue) -2e+03)) "TraceTypeQuery1" false (Utilities|Array|MakeArray _asbp_third_person_character) "None"))
    (if _returnvalue_3
      (Development|PrintString (Utilities|String|EnumtoString (Collision|GetSurfaceType _outhit)))
      (switch Utilities|FlowControl|Switch|SwitchonEPhysicalSurface (Collision|GetSurfaceType _outhit)
        (:SurfaceType_Default
          (Audio|PlaySoundatLocation "/Game/SFX/Footsteps/AudioFiles/Footsteps_Rock/Footsteps_Rock_Run/Step_Rock_Cue.Step_Rock_Cue" _returnvalue_2 "0, 0, 0" 1.0 1.0 0.0 0 0 0 0 :!label _label))
        (:SurfaceType1
          (Audio|PlaySoundatLocation "/Game/SFX/Footsteps/AudioFiles/Footsteps_Grass/Footsteps_Grass_Run/Step_Grass_Cue.Step_Grass_Cue" _returnvalue_2 "0, 0, 0" 1.0 1.0 0.0 0 0 0 0))
        (:SurfaceType2
          (Audio|PlaySoundatLocation "/Game/SFX/Footsteps/AudioFiles/Footsteps_DirtyGround/Footsteps_DirtyGround_Run/Step_DirtyGround_Cue.Step_DirtyGround_Cue" _returnvalue_2 "0, 0, 0" 1.0 1.0 0.0 0 0 0 0))
        (:SurfaceType3
          (Audio|PlaySoundatLocation "/Game/SFX/Footsteps/AudioFiles/Footsteps_Gravel/Footsteps_Gravel_Run/Step_Gravel_Cue.Step_Gravel_Cue" _returnvalue_2 "0, 0, 0" 1.0 1.0 0.0 0 0 0 0))
        (:SurfaceType4
          (Audio|PlaySoundatLocation "/Game/SFX/Footsteps/AudioFiles/Footsteps_Leaves/Footsteps_Leaves_Run/Step_Leaves_Cue.Step_Leaves_Cue" _returnvalue_2 "0, 0, 0" 1.0 1.0 0.0 0 0 0 0))
        (:SurfaceType5
          (Audio|PlaySoundatLocation "/Game/SFX/Footsteps/AudioFiles/Footsteps_Metal/Footsteps_Metal_Run/Step_Metal_Cue.Step_Metal_Cue" _returnvalue_2 "0, 0, 0" 1.0 1.0 0.0 0 0 0 0))
        (:SurfaceType6
          (Audio|PlaySoundatLocation "/Game/SFX/Footsteps/AudioFiles/Footsteps_Mud/Footsteps_Mud_Run/Step_Mud_Cue.Step_Mud_Cue" _returnvalue_2 "0, 0, 0" 1.0 1.0 0.0 0 0 0 0))
        (:SurfaceType7
          (goto _label))
        (:SurfaceType8
          (Audio|PlaySoundatLocation "/Game/SFX/Footsteps/AudioFiles/Footsteps_Sand/Footsteps_Sand_Run/Step_Sand_Cue.Step_Sand_Cue" _returnvalue_2 "0, 0, 0" 1.0 1.0 0.0 0 0 0 0))
        (:SurfaceType9
          (Audio|PlaySoundatLocation "/Game/SFX/Footsteps/AudioFiles/Footsteps_Snow/Footsteps_Snow_Run/Step_Snow_Cue.Step_Snow_Cue" _returnvalue_2 "0, 0, 0" 1.0 1.0 0.0 0 0 0 0))
        (:SurfaceType10
          (Audio|PlaySoundatLocation "/Game/SFX/Footsteps/AudioFiles/Footsteps_Tile/Footsteps_Tile_Run/Step_Tile_Cue.Step_Tile_Cue" _returnvalue_2 "0, 0, 0" 1.0 1.0 0.0 0 0 0 0))
        (:SurfaceType11
          (Audio|PlaySoundatLocation "/Game/SFX/Footsteps/AudioFiles/Footsteps_Water/Footsteps_Water_Run/Step_Water_Cue.Step_Water_Cue" _returnvalue_2 "0, 0, 0" 1.0 1.0 0.0 0 0 0 0)))
      (return false))))